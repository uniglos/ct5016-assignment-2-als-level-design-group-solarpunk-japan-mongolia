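; BP_BulletTrain is a Level 1 actor that moves a train along a referenced spline.
; On BeginPlay, MoveTrain sets the timeline play rate from TimeToComplete and plays it.
; Each update maps the timeline's float to a distance along the spline and sets the actor's world location there without sweep, leaving rotation unchanged.
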(event `self.ReceiveBeginPlay`
  (`self.MoveTrain`))

(event `MoveTrain`
  (bind _spline (`/Game/Blueprints/Level1/BP_BulletTrainSpline.Spline` (`self.SplineRef`)))
  (`TimelineComponent.SetPlayRate` (`self.Timeline`) (/ 1.0 (`self.TimeToComplete`)))
  (bind (_direction _trainfloat) (`Timeline|Timeline`)
    (:`Update`
      (`self.K2_SetActorLocation` (`SplineComponent.GetLocationAtDistanceAlongSpline` _spline (`KismetMathLibrary.Lerp` 0.0 (`SplineComponent.GetSplineLength` _spline) _trainfloat) "World")))))

(fn `UserConstructionScript`)