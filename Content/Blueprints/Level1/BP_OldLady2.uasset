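; Elderly lady NPC for Level 1 that the player can talk to for voiced dialogue.
; Entering her box shows the talk prompt, enables input and unregisters the player's AI perception stimuli; leaving only re-registers them.
; Interact picks one of two chained audio sequences based on the player's HelpedLady flag, with only the not-helped branch disabling input and clearing the prompt.
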(event `self.Box.OnComponentBeginOverlap`
  (params (OverlappedComponent :type "PrimitiveComponent Object Reference") (OtherActor :type "Actor Object Reference") (OtherComp :type "PrimitiveComponent Object Reference") (OtherBodyIndex :type Integer) (bFromSweep :type Boolean) (SweepResult :type "HitResult Structure (by ref)"))
  (bind _asbp_player (cast `/Game/Blueprints/BP_Player` OtherActor))
  (`self.EnableInput` (`GameplayStatics.GetPlayerController` 0))
  (set `/Game/Blueprints/BP_Player.CurrentInteractText` "E - Talk to Elderly Lady" _asbp_player)
  (`AIPerceptionStimuliSourceComponent.UnregisterFromPerceptionSystem` (`/Game/Blueprints/BP_Player.AIPerceptionStimuliSource` _asbp_player)))

(event `InputAction|Interact`
  (params (Key :type "Key Structure"))
  (:`Pressed`
    (if (`/Game/Blueprints/BP_Player.HelpedLady` (stale `self.Box.OnComponentBeginOverlap` _asbp_player))
      (`AudioComponent.Play` (`self.Audio3`) 0.0)
      (else
        (`self.DisableInput` (`GameplayStatics.GetPlayerController` 0))
        (`AudioComponent.Play` (`self.Audio`) 0.0)
        (set `/Game/Blueprints/BP_Player.CurrentInteractText` " " (stale `self.Box.OnComponentBeginOverlap` _asbp_player))))))

(event `self.Audio.OnAudioFinished`
  (`AudioComponent.Play` (`self.Audio1`) 0.0))

(event `self.Audio3.OnAudioFinished`
  (`AudioComponent.Play` (`self.Audio4`) 0.0))

(event `self.Audio1.OnAudioFinished`
  (`AudioComponent.Play` (`self.Audio2`) 0.0))

(event `self.Box.OnComponentEndOverlap`
  (params (OverlappedComponent :type "PrimitiveComponent Object Reference") (OtherActor :type "Actor Object Reference") (OtherComp :type "PrimitiveComponent Object Reference") (OtherBodyIndex :type Integer))
  (bind _asbp_player (cast `/Game/Blueprints/BP_Player` OtherActor))
  (`AIPerceptionStimuliSourceComponent.RegisterWithPerceptionSystem` (`/Game/Blueprints/BP_Player.AIPerceptionStimuliSource` _asbp_player)))

(fn `UserConstructionScript`)